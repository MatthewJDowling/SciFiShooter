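; Base first-person weapon actor that attaches to the player's grip socket and spawns a third-person view model.
; While firing, Tick dispatches by fire mode and shot type, using DoOnce gates and Delays for single, three-shot burst and automatic hitscan.
; Hitscan traces from the camera, playing sound and animation and applying damage; projectiles are supported only in single-fire mode, without a gate.
; Ammo is initialised but never consumed, and Tick prints the firing state.
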(event `self.ReceiveTick`
  (params (DeltaSeconds :type "Float (single-precision)"))
  (bind _isfiring (`self.IsFiring`))
  ;[1 1 1] Firing the Weapon
  (`KismetSystemLibrary.PrintString` (`KismetStringLibrary.Conv_BoolToString` _isfiring) true false (struct :`R` 0.428066 :`G` 1.0 :`A` 1.0) 0.0)
  (if _isfiring
    (`self.MouseInput`)))

(event `StartFiring`
  ;[1 1 1] Firing the Weapon
  (set `self.IsFiring` true))

(event `MouseInput`
  (bind _fburstdelay (`self.FBurstDelay`))
  (switch `/Game/HardLightBP/E_WeaponFireType` (`self.EFireMode`)
    (:`NewEnumerator0`
      ;[1 1 1] Handle Single Fire
      (switch `/Game/HardLightBP/E_WeaponShotType` (`self.EShotType`)
        (:`NewEnumerator0`
          (`self.FireActorProjectile`))
        (:`NewEnumerator1`
          (`/Engine/EditorBlueprintResources/StandardMacros.DoOnce` false :!label _label
            (:`Completed`
              (`self.FireHitScanShot`)
              (set `self.IsFiring` false))))))
    (:`NewEnumerator1`
      ;[1 1 1] Burst Fire
      (switch `/Game/HardLightBP/E_WeaponShotType` (`self.EShotType`)
        (:`NewEnumerator1`
          (`/Engine/EditorBlueprintResources/StandardMacros.DoOnce` false :!label _label_2
            (:`Completed`
              (set `self.IsFiring` false)
              (`KismetSystemLibrary.Delay` _fburstdelay)
              (`self.FireHitScanShot`)
              (`KismetSystemLibrary.Delay` _fburstdelay)
              (`self.FireHitScanShot`)
              (`KismetSystemLibrary.Delay` (`self.FBurstDelay`))
              (`self.FireHitScanShot`))))))
    (:`NewEnumerator2`
      ;[1 1 1] Handle Automatic Fire
      (switch `/Game/HardLightBP/E_WeaponShotType` (`self.EShotType`)
        (:`NewEnumerator1`
          (`KismetSystemLibrary.Delay` 0.2)
          (`self.FireHitScanShot`))))))

(event `StopFiring`
  ;[1 1 1] Stop Firing Burst and Single Fires
  (switch `/Game/HardLightBP/E_WeaponFireType` (`self.EFireMode`)
    (:`NewEnumerator0`
      (goto _label :!via `Reset`))
    (:`NewEnumerator1`
      (goto _label_2 :!via `Reset`))))

(event `self.ReceiveBeginPlay`
  (bind _asfirst_person_character (cast `/Game/HardLightBP/FirstPersonCharacter` (`self.GetOwner`)))
  (`self.SetOwner` _asfirst_person_character)
  (`|SpawnActorFromClass` (`self.ThirdPersonViewModel`) (`self.GetTransform` _asfirst_person_character) "AlwaysSpawn" "OverrideRootScale" (`self.GetOwner`) _asfirst_person_character))

(fn `EquipToPlayer`
  (params (OwningPlayer :type "/Game/HardLightBP/FirstPersonCharacter Object Reference"))
  (`SceneComponent.K2_AttachToComponent` (`self.DefaultSceneRoot`) (`/Game/HardLightBP/FirstPersonCharacter.FirstPersonMesh` OwningPlayer) "GripPoint" "SnapToTarget" "SnapToTarget" "KeepRelative" false))

(fn `FireActorProjectile`
  (bind _instigator (`self.Instigator`))
  (bind _firstpersoncamera (`/Game/HardLightBP/FirstPersonCharacter.FirstPersonCamera` (cast `/Game/HardLightBP/FirstPersonCharacter` (`self.Instigator`) :!pure true)))
  (bind _returnvalue (`SceneComponent.K2_GetComponentLocation` _firstpersoncamera))
  (bind _returnvalue_2 (`|SpawnActorFromClass` (`self.AProjectileType`) (`KismetMathLibrary.MakeTransform` _returnvalue (`KismetMathLibrary.FindLookAtRotation` _returnvalue (+ _returnvalue (`KismetMathLibrary.Conv_RotatorToVector` (`SceneComponent.K2_GetComponentRotation` _firstpersoncamera))))) "AlwaysSpawn" "OverrideRootScale" _instigator _instigator))
  (bind _asfirst_person_projectile (cast `/Game/HardLightBP/FirstPersonProjectile` _returnvalue_2))
  (set `Actor.Instigator` (`self.Instigator`) _asfirst_person_projectile))

(fn `FireHitScanShot`
  (bind _firstpersoncamera (`/Game/HardLightBP/FirstPersonCharacter.FirstPersonCamera` (cast `/Game/HardLightBP/FirstPersonCharacter` (`self.Instigator`) :!pure true)))
  (bind _returnvalue (`SceneComponent.K2_GetComponentLocation` _firstpersoncamera))
  (bind _outhit (`KismetSystemLibrary.LineTraceSingle` :`Start` _returnvalue :`End` (+ _returnvalue (* (`KismetMathLibrary.Conv_RotatorToVector` (`SceneComponent.K2_GetComponentRotation` _firstpersoncamera)) (`self.FWeaponRange`))) :`TraceChannel` "TraceTypeQuery1" :`DrawDebugType` "ForDuration"))
  (`GameplayStatics.PlaySound2D` "/Game/FirstPerson/Audio/FirstPersonTemplateWeaponFire02.FirstPersonTemplateWeaponFire02" 0.25 1.0 0.0 null null)
  (`/Game/HardLightBP/FirstPersonCharacter.PlayFireAnimation` (cast `/Game/HardLightBP/FirstPersonCharacter` (`self.GetOwner`) :!pure true) (`self.Fire Animation`))
  (bind (_bblockinghit _binitialoverlap _time _distance _location _impactpoint _normal _impactnormal _physmat _hitactor) (`GameplayStatics.BreakHitResult` _outhit))
  (if (`Actor.bCanBeDamaged` _hitactor)
    (`GameplayStatics.ApplyDamage` _hitactor (`self.FWeaponDamage`) null (`self.GetOwner`))))

(fn `UserConstructionScript`
  (set `self.IntCurrentAmmo` (`self.IntMaxAmmo`)))